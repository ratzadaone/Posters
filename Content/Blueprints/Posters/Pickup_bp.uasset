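; Pickup_bp is a collectible poster actor that shows a pickup prompt and adds to the player's collected posters count.
; An overlap interface event toggles the TopDownController's pickup widget and fills it with the actor name and TextRender text.
; The pickup interface event increments the count by parsing the player widget's displayed text, then destroys the actor.
; Built-in overlap events are empty, and older widget-search and mesh-setting logic is left disconnected.
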(event EventBeginPlay
  (Variables|Default|SetPlayerControllerRef (.AsTop%20Down%20Controller (Utilities|Casting|CastToTopDownController (Game|GetPlayerController 0)))))

(event Collision|EventActorBeginOverlap
  (params (OtherActor :type Actor%20Object%20Reference)))

(event Collision|EventActorEndOverlap
  (params (OtherActor :type Actor%20Object%20Reference)))

(event EventSomeFunctioninInterface
  (bind _playercontrollerref (Variables|Default|GetPlayerControllerRef))
  (bind _playerwidget (Variables|/Game/Blueprints/Player/TopDownController.TopDownController_C|GetPlayerWidget _playercontrollerref))
  (bind _posterscollected (Variables|/Game/Blueprints/Posters/PlayerUI_widget.PlayerUI_widget_C|GetPostersCollected _playerwidget))
  (Development|PrintString (Utilities|String|Append "Actor: " (Utilities|GetObjectName self) " Pick_Up  blueprint recieved something 2Do"))
  (Rendering|Components|TextRender|SetText _posterscollected (Utilities|Text|ToText(Integer) (+ (Math|Conversions|ToInteger(Byte) (Utilities|String|ToString(Text) (Class|TextBlock|GetText _posterscollected))) 1)))
  (Actor|DestroyActor))

(event EventAnotherOneforOverlap
  (params (StartTrueEndFalse :type Boolean))
  (bind _playercontrollerref (Variables|Default|GetPlayerControllerRef))
  (bind _pickupwidget (Variables|/Game/Blueprints/Player/TopDownController.TopDownController_C|GetPickupWidget _playercontrollerref))
  (Development|PrintString (Utilities|String|Append "Player Overlapped: " (Utilities|GetObjectName self)))
  (if StartTrueEndFalse
    (Widget|SetVisibility _pickupwidget "Visible")
    ;[1 1 1] Only Works for One
    ; maybe better set a variable inside so it shows nicer
    (Rendering|Components|TextRender|SetText (Variables|/Game/Blueprints/Posters/Pickup_widget.Pickup_widget_C|GetOverlappedPoster _pickupwidget) (Utilities|Text|ToText(String) (Utilities|String|Append (Utilities|GetObjectName self) " " (Utilities|String|ToString(Text) (Variables|/Script/Engine.TextRenderComponent|GetText (Variables|Default|GetTextRender))))))
    (else
      (Widget|SetVisibility _pickupwidget "Hidden"))))

(fn ConstructionScript)